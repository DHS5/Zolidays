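; World pickup actor that gives a player a firearm, hand weapon, projectile or ammo, configured from the class defaults of its PickableObjectComponent class.
; Construction sets the mesh, physics and quantity text.
; Pickup tops up ammo or a matching component, otherwise drops the same-type object and adds the component at runtime, destroying itself or refreshing text if adding fails.
; After a hit, sphere overlap stops physics.
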(event OnComponentBeginOverlap(SphereCollision)
  (params (OverlappedComponent :type Primitive%20Component%20Object%20Reference) (OtherActor :type Actor%20Object%20Reference) (OtherComp :type Primitive%20Component%20Object%20Reference) (OtherBodyIndex :type Integer) (bFromSweep :type Boolean) (SweepResult :type Hit%20Result%20Structure%20%28by%20ref%29))
  ;[1 1 1] Stop physics when overlapped, if already hit the ground
  (Physics|SetSimulatePhysics (Variables|Default|GetStaticMesh) false)
  (Collision|SetCollisionResponsetoChannel (Variables|Default|GetStaticMesh) "ECC_Pawn" "ECR_Block"))

(event OnComponentHit(StaticMesh)
  (params (HitComponent :type Primitive%20Component%20Object%20Reference) (OtherActor :type Actor%20Object%20Reference) (OtherComp :type Primitive%20Component%20Object%20Reference) (NormalImpulse :type Vector :default "0, 0, 0") (Hit :type Hit%20Result%20Structure%20%28by%20ref%29))
  ;[1 1 1] Stop physics when overlapped, if already hit the ground
  (Collision|SetCollisionResponsetoChannel (Variables|Default|GetSphereCollision) "ECC_Pawn" "ECR_Overlap"))

(event Custom|Update%20Text
  (Rendering|Components|TextRender|SetText (Variables|Default|GetTextRender) (Utilities|Text|MakeLiteralText (Utilities|Text|ToText(String) (Utilities|String|Append "T<br>" (Utilities|Select :Index (Variables|Object|GetObject%20Type) :NewEnumerator0 "Ammo : " :NewEnumerator1 "" :NewEnumerator2 "Quantity : " :NewEnumerator3 "Ammo :" :NewEnumerator4 "") (Utilities|Select :Index (Variables|Object|GetObject%20Type) :NewEnumerator0 (Utilities|String|ToString(Integer) (Variables|Quantity|GetAmmo%20Quantity)) :NewEnumerator1 "" :NewEnumerator2 (Utilities|String|ToString(Integer) (Variables|Quantity|GetPickup%20Quantity)) :NewEnumerator3 (Utilities|String|ToString(Integer) (Variables|Quantity|GetAmmo%20Quantity)) :NewEnumerator4 ""))))))

(event EventPickup
  (params (Picking%20Player :type BP%20First%20Person%20Character%20Object%20Reference))
  (bind _pickableobject_component (Variables|Object|GetPickableObject%20Component))
  (bind (_object_icon _use_delay _relativelocation _relativerotation _relativescale3d) (Utilities|GetClassDefaults _pickableobject_component))
  ;[1 1 1] Add a Pickable Object Component to the player
  (Variables|Default|SetPicking%20Player Picking%20Player)
  (if (Utilities|Enum|Equal(Enum) (Variables|Object|GetObject%20Type) "NewEnumerator3")
    (bind _take_ammos (Default|AddAmmos (Variables|Default|GetPicking%20Player) (Variables|Quantity|GetAmmo%20Quantity) self))
    (if _take_ammos
      (Actor|DestroyActor :!label _label)
      (else
        (CallFunction|UpdateText :!label _label_2)))
    (else
      (Utilities|IsValid (Actor|GetComponentbyClass (Variables|Default|GetPicking%20Player) (Variables|Object|GetPickableObject%20Component))
        (:Is%20Valid
          (bind _take_ammos_2 (Default|AddAmmos (Actor|GetComponentbyClass (Variables|Default|GetPicking%20Player) (Variables|Object|GetPickableObject%20Component)) self (Variables|Quantity|GetPickup%20Quantity) (Variables|Quantity|GetAmmo%20Quantity)))
          (if _take_ammos_2
            (goto _label)
            (else
              (goto _label_2))))
        (:Is%20Not%20Valid
          (Utilities|FlowControl|Sequence
            (:then_0
              ;;[1 1 1] Drop Previous Object
              (switch Utilities|FlowControl|Switch|SwitchonE_PickableObjectType (Variables|Object|GetObject%20Type)
                (:NewEnumerator0
                  (Utilities|IsValid (Variables|/Game/FirstPerson/Blueprints/BP_FirstPersonCharacter.BP_FirstPersonCharacter_C|GetFirearm (Variables|Default|GetPicking%20Player))
                    (:Is%20Valid
                      (Default|DropObject (Variables|/Game/FirstPerson/Blueprints/BP_FirstPersonCharacter.BP_FirstPersonCharacter_C|GetFirearm (Variables|Default|GetPicking%20Player)) true))))
                (:NewEnumerator1
                  (Utilities|IsValid (Variables|/Game/FirstPerson/Blueprints/BP_FirstPersonCharacter.BP_FirstPersonCharacter_C|GetHand%20Weapon (Variables|Default|GetPicking%20Player))
                    (:Is%20Valid
                      (Default|DropObject (Variables|/Game/FirstPerson/Blueprints/BP_FirstPersonCharacter.BP_FirstPersonCharacter_C|GetHand%20Weapon (Variables|Default|GetPicking%20Player)) true))))
                (:NewEnumerator2
                  (Utilities|IsValid (Variables|/Game/FirstPerson/Blueprints/BP_FirstPersonCharacter.BP_FirstPersonCharacter_C|GetProjectile (Variables|Default|GetPicking%20Player))
                    (:Is%20Valid
                      (Default|DropObject (Variables|/Game/FirstPerson/Blueprints/BP_FirstPersonCharacter.BP_FirstPersonCharacter_C|GetProjectile (Variables|Default|GetPicking%20Player)) true))))))
            (:then_1
              ;;[1 1 1] Add New Component
              (bind _returnvalue (Game|AddComponentbyClass (Variables|Default|GetPicking%20Player) _pickableobject_component false (Math|Transform|MakeTransform _relativelocation _relativerotation _relativescale3d)))
              (Default|CreateComponent _returnvalue (Variables|Quantity|GetAmmo%20Quantity) (Variables|Quantity|GetPickup%20Quantity) (Utilities|GetClass self) (Transformation|GetRelativeTransform (Variables|Default|GetStaticMesh)))
              (goto _label))))))))

(fn ConstructionScript
  (bind _pickableobject_component (Variables|Object|GetPickableObject%20Component))
  (bind (_object_type _bisselected _noise_loudness _object_icon _use_delay _staticmesh) (Utilities|GetClassDefaults _pickableobject_component))
  (Variables|Object|SetObject%20Type _object_type)
  (Utilities|IsValid _staticmesh
    (:Is%20Valid
      (Components|StaticMesh|SetStaticMesh (Variables|Default|GetStaticMesh) _staticmesh)
      (Physics|SetSimulatePhysics (Variables|Default|GetStaticMesh) true)
      (CallFunction|UpdateText))))