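; Zombie AI character that senses the player, attacks in melee and ragdolls on death.
; PawnSensing sight and hearing write to Blackboard keys, with retriggerable delays clearing them and louder noises overriding current ones.
; Sightings, heard noises and damage trigger Alert, which changes sensing range and emits noise.
; Externally triggered events switch walk/run speed, update attack state by distance, and box-trace from the head to damage and knock back the player.
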(event OnSeePawn(PawnSensing)
  (params (Pawn :type Pawn%20Object%20Reference))
  ;[0 0.5169 1] See Player
  (if (== Pawn (Variables|Default|GetPlayer))
    (CallFunction|SeePlayer true)
    (Utilities|FlowControl|Sequence
      (:then_0
        (bind _output_get (Variables|State|SetDistanceToPlayer (Transformation|GetDistanceTo (Variables|Default|GetPlayer))))
        (Variables|State|SetbIsAttacking (<= _output_get (Variables|Characteristics|GetMax%20Attack%20Distance))))
      (:then_1
        (Utilities|FlowControl|RetriggerableDelay (+ (Variables|/Script/AIModule.PawnSensingComponent|GetSensingInterval (Variables|Default|GetPawnSensing)) 0.1 0.0))
        (CallFunction|SeePlayer false)
        (Variables|State|SetbIsAttacking false)))))

(event OnHearNoise(PawnSensing)
  (params (Instigator :type Pawn%20Object%20Reference) (Location :type Vector%20%28by%20ref%29 :default "0, 0, 0") (Volume :type Float%20%28single-precision%29))
  ;[0.1696 1 0] Heard Noise
  (if (or (not (Variables|State|GetbHeardNoise)) (>= Volume (Variables|Sensing|GetNoise%20Volume)))
    (Variables|Sensing|SetNoise%20Location Location)
    (bind _output_get (Variables|Sensing|SetNoise%20Volume Volume))
    (CallFunction|HearNoise true)
    (Utilities|FlowControl|RetriggerableDelay (* _output_get (Variables|Sensing|GetNoise%20Interest%20Duration)))
    (CallFunction|HearNoise false)))

(event Custom|Dead
  (bind _mesh (Variables|Character|GetMesh))
  ;[0 0 0] Dead
  (Default|CallDied)
  (Variables|State|SetbIsAlive false)
  (Class|Pawn|PawnMakeNoise 1.0 "0, 0, 0" true 0)
  (Collision|SetCollisionEnabled _mesh "PhysicsOnly")
  (Physics|SetSimulatePhysics _mesh true)
  (Collision|SetCollisionEnabled (Variables|Collision|GetCapsuleComponent) "NoCollision")
  (Components|DestroyComponent (Variables|Default|GetPawnSensing))
  (Variables|State|SetbIsAttacking false)
  (Variables|State|SetbSeePlayer false))

(event Custom|OnTakeAnyDamage_Event
  (params (DamagedActor :type Actor%20Object%20Reference) (Damage :type Float%20%28single-precision%29) (DamageType :type Damage%20Type%20Object%20Reference) (InstigatedBy :type Controller%20Object%20Reference) (DamageCauser :type Actor%20Object%20Reference))
  ;[1 0 0] Damage
  (bind _output_get (Variables|Characteristics|SetHealth (- (Variables|Characteristics|GetHealth) Damage)))
  (if (<= _output_get 0.0)
    (CallFunction|Dead)
    (else
      (CallFunction|Alert true (Variables|Noise|GetDamage%20Noise%20Loudness)))))

(event Custom|Attack
  (bind _mesh (Variables|Character|GetMesh))
  (bind _returnvalue (Transformation|GetSocketLocation _mesh "Head"))
  ;[1 0.2843 0] Attack
  (bind _outhit (Class|KismetSystemLibrary|BoxTraceSingleforObjects _returnvalue (+ _returnvalue (* (Variables|Hit|GetHit%20Distance) (Math|Vector|GetUnitDirection(Vector) _returnvalue (Transformation|GetActorLocation (Variables|Default|GetPlayer))))) "25.000000,25.000000,25.000000" (Transformation|GetActorRotation) (Utilities|Array|MakeArray "ObjectTypeQuery3") false 0 "ForDuration" true))
  (if (== (.HitActor (Collision|BreakHitResult _outhit)) (Game|GetPlayerCharacter 0))
    (Game|Damage|ApplyDamage (.HitActor (Collision|BreakHitResult _outhit)) (Variables|Hit|GetHit%20Damage) 0 0)
    (Class|Actor|MakeNoise (Variables|Hit|GetHit%20Noise) 0 (Transformation|GetActorLocation) (Variables|Noise|GetNoise%20Range) "None")
    (bind _ascharacter (Utilities|Casting|CastToCharacter (.HitActor (Collision|BreakHitResult _outhit))))
    (Physics|AddImpulse (Variables|/Script/Engine.Character|GetCharacterMovement _ascharacter) (Math|Vector|MakeVector (.x (* (Math|Vector|Normalize (- (Transformation|GetActorLocation (.HitActor (Collision|BreakHitResult _outhit))) (Transformation|GetActorLocation))) (Variables|Hit|GetHit%20Impulse))) (.y (* (Math|Vector|Normalize (- (Transformation|GetActorLocation (.HitActor (Collision|BreakHitResult _outhit))) (Transformation|GetActorLocation))) (Variables|Hit|GetHit%20Impulse))) 1e+01) true)))

(event Custom|Target
  (params (State :type Boolean))
  (bind _charactermovement (Variables|Character|GetCharacterMovement))
  ;[0 1 0.8583] Target
  (bind _output_get (Variables|State|SetbHasTarget State))
  (if _output_get
    (Variables|/Script/Engine.CharacterMovementComponent|SetMaxWalkSpeed _charactermovement (Variables|Characteristics|GetRun%20Speed))
    (else
      (Variables|/Script/Engine.CharacterMovementComponent|SetMaxWalkSpeed _charactermovement (Variables|Characteristics|GetWalk%20Speed)))))

(event Custom|Alert
  (params (State :type Boolean) (Noise%20Loudness :type Float%20%28double-precision%29))
  ;[1 0 0] Alert
  (bind _pawnsensing (Variables|Default|GetPawnSensing)
    (:then
      (if State
        (Variables|/Script/AIModule.PawnSensingComponent|SetSightRadius _pawnsensing (Variables|Sensing|GetAlert%20Sight%20Distance))
        (Class|PawnSensingComponent|SetPeripheralVisionAngle _pawnsensing (Variables|Sensing|GetAlert%20Vision%20Angle))
        (Class|Actor|MakeNoise Noise%20Loudness 0 (Transformation|GetActorLocation) (Variables|Noise|GetNoise%20Range) "None")
        (else
          (Variables|/Script/AIModule.PawnSensingComponent|SetSightRadius _pawnsensing (Variables|Sensing|GetMax%20Sight%20Distance))
          (Class|PawnSensingComponent|SetPeripheralVisionAngle _pawnsensing (Variables|Sensing|GetAlert%20Vision%20Angle)))))
    (:else)))

(event Custom|Feel%20Player
  (params (State :type Boolean))
  ;[1 1 1] Feel Player
  (if State
    (bind _output_get (Variables|State|SetDistanceToPlayer (Transformation|GetDistanceTo (Variables|Default|GetPlayer))))
    (Variables|State|SetbIsAttacking (<= _output_get (Variables|Characteristics|GetMax%20Attack%20Distance)))
    (else
      (Variables|State|SetbIsAttacking false))))

(event EventBeginPlay
  (bind (_returnvalue _returnvalue2) (CallFunction|BlackboardData "Player"))
  (EventDispatchers|BindEventtoOnTakeAnyDamage (delegate Custom|OnTakeAnyDamage_Event))
  (bind _output_get (Variables|Default|SetPlayer (Game|Player|GetPlayerPawn 0)))
  (AI|Components|Blackboard|SetValueasObject _returnvalue _returnvalue2 _output_get))

(fn ConstructionScript
  (bind _pawnsensing (Variables|Default|GetPawnSensing))
  (Variables|Characteristics|SetHealth (Variables|Characteristics|GetMax%20Health))
  (Variables|/Script/AIModule.PawnSensingComponent|SetSightRadius _pawnsensing (Variables|Sensing|GetMax%20Sight%20Distance))
  (Class|PawnSensingComponent|SetPeripheralVisionAngle _pawnsensing (Variables|Sensing|GetVision%20Angle))
  (Variables|/Script/AIModule.PawnSensingComponent|SetHearingThreshold _pawnsensing (Variables|Sensing|GetMax%20Hearing%20Distance))
  (Variables|/Script/Engine.CharacterMovementComponent|SetMaxWalkSpeed (Variables|Character|GetCharacterMovement) (Variables|Characteristics|GetWalk%20Speed)))

(fn BlackboardData
  (params (KeyName :type Name))
  (bind _self self)
  (bind _returnvalue (AI|GetAIController _self))
  (bind _returnvalue_2 (AI|GetBlackboard _returnvalue))
  (Utilities|IsValid _returnvalue_2
    (:Is%20Valid
      _)
    (:Is%20Not%20Valid
      (Development|PrintString "Not Valid")))
  (return _returnvalue_2 (Utilities|Name|MakeLiteralName KeyName)))

(fn SeePlayer
  (params (State :type Boolean))
  (bind (_returnvalue _returnvalue2) (CallFunction|BlackboardData "LastSeenLocation"))
  (bind (_returnvalue_2 _returnvalue2_2) (CallFunction|BlackboardData "SeePlayer"))
  (bind _output_get (Variables|State|SetbSeePlayer State))
  (AI|Components|Blackboard|SetValueasBool _returnvalue_2 _returnvalue2_2 _output_get)
  (CallFunction|Alert State (Variables|Noise|GetSeePlayer%20Noise%20Loudness))
  (AI|Components|Blackboard|SetValueasVector _returnvalue _returnvalue2 (Transformation|GetActorLocation (Variables|Default|GetPlayer))))

(fn HearNoise
  (params (State :type Boolean))
  (bind (_returnvalue _returnvalue2) (CallFunction|BlackboardData "HearNoise"))
  (bind (_returnvalue_2 _returnvalue2_2) (CallFunction|BlackboardData "NoiseLocation"))
  (bind _output_get (Variables|State|SetbHeardNoise State))
  (AI|Components|Blackboard|SetValueasBool _returnvalue _returnvalue2 _output_get)
  (CallFunction|Alert State (Variables|Noise|GetAlert%20Noise%20Loudness))
  (if State
    (AI|Components|Blackboard|SetValueasVector _returnvalue_2 _returnvalue2_2 (Variables|Sensing|GetNoise%20Location))))