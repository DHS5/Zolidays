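; BP_ZombieSpawn is a placeable spawner that creates a horde of zombies at level start, gated by the game mode's difficulty.
; If difficulty meets its minimum, the horde size scales from an average plus a difficulty multiplier, with random variation.
; Each zombie spawns at a random navigable point within the radius and receives a reference back to its spawner.
; The construction script sizes a sphere component to match that radius.
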(event Custom|Spawn
  ;[0 0.6093 1] Spawn
  (bind _randomlocation (Class|NavigationSystemV1|GetRandomLocationinNavigableRadius (Transformation|GetActorLocation) (Variables|Sphere|GetSphere%20Radius) 0 0))
  (bind _returnvalue (Game|SpawnActorfromClass (Variables|Zombie|GetZombie%20Character) (Math|Transform|MakeTransform _randomlocation "0, 0, 0" "1.000000,1.000000,1.000000") "AdjustIfPossibleButAlwaysSpawn" 0 0))
  (Variables|/Game/Zombie/BP_ZombieCharacter.BP_ZombieCharacter_C|SetZombieSpawn _returnvalue self))

(event Custom|Spawn%20Hord
  (params (Average%20Number :type Integer))
  ;[0 0.1266 1] Spawn Hord
  (Variables|Sphere|SetSphere%20Origin (Transformation|GetActorLocation))
  (for _index (range 1 (- (+ Average%20Number (Math|Random|RandomInteger (* (Variables|Zombie|GetVariation%20Spawn%20Number) 2))) (Variables|Zombie|GetVariation%20Spawn%20Number)))
    (CallFunction|Spawn)))

(event EventBeginPlay
  ;[1 1 1] Begin Play
  (bind _asbp_first_person_game_mode (Utilities|Casting|CastToBP_FirstPersonGameMode (Game|GetGameMode)))
  (if (<= (Math|Conversions|ToInteger(Byte) (Variables|Zombie|GetMinimum%20Difficulty)) (Math|Conversions|ToInteger(Byte) (Variables|/Game/FirstPerson/Blueprints/BP_FirstPersonGameMode.BP_FirstPersonGameMode_C|GetGame%20Difficulty _asbp_first_person_game_mode)))
    (CallFunction|SpawnHord (+ (Variables|Zombie|GetAverage%20Spawn%20Number) (* (Math|Conversions|ToInteger(Byte) (Variables|/Game/FirstPerson/Blueprints/BP_FirstPersonGameMode.BP_FirstPersonGameMode_C|GetGame%20Difficulty _asbp_first_person_game_mode)) (Variables|Zombie|GetDifficulty%20Spawn%20Multiplier))))))

(fn ConstructionScript
  (Components|Sphere|SetSphereRadius (Variables|Default|GetSphere) (Variables|Sphere|GetSphere%20Radius) true))